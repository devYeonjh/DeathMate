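; Paper2D player character Blueprint that handles jump input and drives flipbook animation.
; Enhanced Input IA_Jump starts and stops the jump, while Tick calls UdateAnimation every frame.
; That function picks Run or Idle on the ground by speed, and an airborne flipbook by vertical velocity.
; The airborne names look inverted: fast descent shows JumpRise, and all other airborne motion shows Fall.
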(event Input|EnhancedActionEvents|EnhancedInputActionIA_Jump
  (params (ActionValue :type Boolean) (ElapsedSeconds :type Float%20%28double-precision%29) (TriggeredSeconds :type Float%20%28double-precision%29) (InputAction :type Input%20Action%20Object%20Reference :default "/Game/DoHoon/Input/Action/IA_Jump.IA_Jump"))
  (:Started
    (Character|Jump))
  (:Completed
    (Character|StopJumping)))

(event EventBeginPlay)

(event Collision|EventActorBeginOverlap
  (params (OtherActor :type Actor%20Object%20Reference)))

(event EventTick
  (params (DeltaSeconds :type Float%20%28single-precision%29))
  (CallFunction|UdateAnimation))

(fn ConstructionScript)

(fn UdateAnimation
  (if (AI|Components|NavMovement|IsMovingonGround (Variables|Character|GetCharacterMovement))
    (if (> (Math|Vector|VectorLength (Transformation|GetVelocity)) 0.0)
      (Sprite|SetFlipbook (Variables|Default|GetSprite) "/Game/DoHoon/PaperAsset/Character/Flipbooks/FB_Player_Run.FB_Player_Run")
      (else
        (Sprite|SetFlipbook (Variables|Default|GetSprite) "/Game/DoHoon/PaperAsset/Character/Flipbooks/FB_Player_Idle.FB_Player_Idle")))
    (elif (< (.z (Transformation|GetVelocity)) -1e+02)
      (Sprite|SetFlipbook (Variables|Default|GetSprite) "/Game/DoHoon/PaperAsset/Character/Flipbooks/FB_Player_JumpRise.FB_Player_JumpRise")
      (else
        (Sprite|SetFlipbook (Variables|Default|GetSprite) "/Game/DoHoon/PaperAsset/Character/Flipbooks/FB_Player_Fall.FB_Player_Fall")))))