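; BP_long_Spike3 is a spike hazard trigger that kills the player and sends them back to the last checkpoint.
; When BP_1P triggers it, it hides the pawn, disables input and spawns a particle burst at the player's location.
; After a short delay it calls RespawnAtCheckpoint on DMGameModeBase, then unhides the pawn and restores input.
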(event EventTriggerEvent
  (params (OtherActor :type Actor%20Object%20Reference))
  (bind _asbp_1p (Utilities|Casting|CastToBP_1P OtherActor))
  (Rendering|SetActorHiddenInGame _asbp_1p true)
  (Input|DisableInput (Game|GetPlayerController 0) 0)
  (Effects|SpawnEmitteratLocation "/Engine/Functions/Engine_MaterialFunctions02/ExampleContent/3dParticleOpacity_Particle.3dParticleOpacity_Particle" (Transformation|GetActorLocation (Game|Player|GetPlayerPawn 0)))
  (Utilities|FlowControl|Delay 1.0)
  (bind _asdmgame_mode_base (Utilities|Casting|CastToDMGameModeBase (Game|GetGameMode)))
  (Class|DMGameModeBase|RespawnatCheckpoint _asdmgame_mode_base)
  (Rendering|SetActorHiddenInGame (Game|Player|GetPlayerPawn 0) false)
  (Input|EnableInput (Game|GetPlayerController 0) 0))

(fn ConstructionScript)