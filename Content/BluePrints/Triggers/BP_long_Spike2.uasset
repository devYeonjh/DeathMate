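; BP_long_Spike2 is a spike hazard trigger that kills the 1P player character and respawns it at the last checkpoint.
; When BP_1P triggers it, it hides the character, disables input and spawns a flipbook death effect at the player's location.
; After a delay equal to the flipbook length, it destroys the effect, calls RespawnAtCheckpoint on DMGameModeBase, then unhides the player and re-enables input.
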(event EventTriggerEvent
  (params (OtherActor :type Actor%20Object%20Reference))
  (bind _asbp_1p (Utilities|Casting|CastToBP_1P OtherActor))
  (Rendering|SetActorHiddenInGame _asbp_1p true)
  (Input|DisableInput (Game|GetPlayerController 0) 0)
  (bind _returnvalue (Game|SpawnActorfromClass "/Game/PaperAssets/VFX/1P/1P_Death_Effect.1P_Death_Effect_C" (Math|Conversions|ToTransform(Vector) (Transformation|GetActorLocation (Game|Player|GetPlayerPawn 0))) "Undefined" "MultiplyWithRoot" 0 0))
  (Utilities|FlowControl|Delay (Class|PaperFlipbookComponent|GetFlipbookLength (Variables|/Script/Paper2D.PaperFlipbookActor|GetRenderComponent _returnvalue)))
  (Actor|DestroyActor _returnvalue)
  (bind _asdmgame_mode_base (Utilities|Casting|CastToDMGameModeBase (Game|GetGameMode)))
  (Class|DMGameModeBase|RespawnatCheckpoint _asdmgame_mode_base)
  (Rendering|SetActorHiddenInGame (Game|Player|GetPlayerPawn 0) false)
  (Input|EnableInput (Game|GetPlayerController 0) 0))

(fn ConstructionScript)