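; Long spike hazard trigger that kills the BP_1P player and sends them back to a checkpoint.
; TriggerEvent disables movement, hides the actor and spawns a death flipbook effect at the player pawn's location.
; After a delay matching the flipbook's length, it destroys the effect, calls RespawnAtCheckpoint on DMGameModeBase, then restores walking and visibility on player pawn 0.
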(event EventTriggerEvent
  (params (OtherActor :type Actor%20Object%20Reference))
  (bind _returnvalue (Game|Player|GetPlayerPawn 0))
  (bind _asbp_1p (Utilities|Casting|CastToBP_1P OtherActor))
  (Pawn|Components|CharacterMovement|DisableMovement (Variables|/Script/Engine.Character|GetCharacterMovement _asbp_1p))
  (Rendering|SetActorHiddenInGame _asbp_1p true)
  (bind _returnvalue_2 (Game|SpawnActorfromClass "/Game/PaperAssets/VFX/1P/1P_Death_Effect.1P_Death_Effect_C" (Math|Conversions|ToTransform(Vector) (Transformation|GetActorLocation (Game|Player|GetPlayerPawn 0))) "Undefined" "MultiplyWithRoot" 0 0))
  (Utilities|FlowControl|Delay (Class|PaperFlipbookComponent|GetFlipbookLength (Variables|/Script/Paper2D.PaperFlipbookActor|GetRenderComponent _returnvalue_2)))
  (Actor|DestroyActor _returnvalue_2)
  (bind _asdmgame_mode_base (Utilities|Casting|CastToDMGameModeBase (Game|GetGameMode)))
  (Class|DMGameModeBase|RespawnatCheckpoint _asdmgame_mode_base)
  (bind _asbp_1p_2 (Utilities|Casting|CastToBP_1P _returnvalue))
  (Pawn|Components|CharacterMovement|SetMovementMode (Variables|/Script/Engine.Character|GetCharacterMovement _asbp_1p_2) "MOVE_Walking" 0)
  (Rendering|SetActorHiddenInGame _returnvalue false))

(fn ConstructionScript)