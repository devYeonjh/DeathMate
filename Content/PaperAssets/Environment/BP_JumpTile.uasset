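; BP_JumpTile is a one-way platform tile that the BP_1P player can pass through from below and land on from above.
; Every Tick runs UpdateCollision, which compares the player's height, less a fixed offset, with the tile's own height.
; The RenderComponent gets query and physics collision while the player is above that threshold, and no collision otherwise.
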(event EventTick
  (params (DeltaSeconds :type Float%20%28single-precision%29))
  (CallFunction|UpdateCollision))

(fn ConstructionScript)

(fn UpdateCollision
  (bind _rendercomponent (Variables|Default|GetRenderComponent))
  (bind _asbp_1p (Utilities|Casting|CastToBP_1P (Game|GetPlayerCharacter 0)))
  (if (> (- (.z (Transformation|GetActorLocation _asbp_1p)) 6e+01) (.z (Transformation|GetActorLocation)))
    (Collision|SetCollisionEnabled _rendercomponent "QueryAndPhysics")
    (else
      (Collision|SetCollisionEnabled _rendercomponent "NoCollision"))))